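; BP_Target is a target actor that jumps to a random nearby position when hit.
; The OnComponentHit event of its Se component prints a debug message, then offsets the actor from its current location by a random vector within a cube centered on it.
; The move neither sweeps nor checks bounds, so the target can drift in any direction, including vertically, over repeated hits.
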(event `self.ReceiveActorBeginOverlap`
  (params (OtherActor :type "Actor Object Reference")))

(event `self.se.OnComponentHit`
  (params (HitComponent :type "PrimitiveComponent Object Reference") (OtherActor :type "Actor Object Reference") (OtherComp :type "PrimitiveComponent Object Reference") (NormalImpulse :type "Vector Structure") (Hit :type "HitResult Structure (by ref)"))
  (`KismetSystemLibrary.PrintString` "target hit")
  (`self.K2_SetActorLocation` (+ (`self.K2_GetActorLocation`) (* (+ (* (`KismetMathLibrary.MakeVector` (`KismetMathLibrary.RandomFloat`) (`KismetMathLibrary.RandomFloat`) (`KismetMathLibrary.RandomFloat`)) (2.0 2.0 2.0)) (-1.0 -1.0 -1.0)) (500.0 500.0 500.0)))))

(fn `UserConstructionScript`)