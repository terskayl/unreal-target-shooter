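; BPC_Shooter is a shooter component that fires BP_Projectile while its NumShots count is above zero.
; Shoot spawns the projectile ahead of and above the given transform, passing it the forward vector and shooter, then decrements the count.
; Each shot sets a looping timer on IncrementShot, which keeps adding shots with no cap or clear in this graph.
; Shoot also prints the current count on every call.
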(fn `IncrementShot`
  (set `self.NumShots` (+ (`self.NumShots`) 1)))

(fn `Shoot`
  (params (ShooterTransform :type "Transform Structure") (ShooterRotation :type "Rotator Structure") (Shooter :type "/Game/FirstPerson/Blueprints/BP_FirstPersonCharacter Object Reference"))
  (bind _returnvalue (`KismetMathLibrary.GetForwardVector` ShooterRotation))
  (bind _numshots (`self.NumShots`))
  (`KismetSystemLibrary.PrintString` (`KismetStringLibrary.Conv_IntToString` _numshots))
  (if (> _numshots 0)
    (`|SpawnActorFromClass` "/Game/BP_Projectile.BP_Projectile_C" (`KismetMathLibrary.ComposeTransforms` (`KismetMathLibrary.ComposeTransforms` ShooterTransform (`KismetMathLibrary.Conv_VectorToTransform` (* _returnvalue (50.0 50.0 50.0)))) (`KismetMathLibrary.Conv_VectorToTransform` (* (`KismetMathLibrary.GetUpVector` (`KismetMathLibrary.TransformRotation` ShooterTransform)) (0.0 0.0 40.0)))) "AlwaysSpawn" "MultiplyWithRoot" null _returnvalue Shooter null)
    (set `self.NumShots` (- (`self.NumShots`) 1))
    (`KismetSystemLibrary.K2_SetTimer` null "IncrementShot" 2.0 true)))